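; Destroyed version of the Scorpion space fighter that blows apart through Chaos physics fields as soon as it spawns.
; On BeginPlay, a radial falloff sized and centered on the BombRadius sphere applies external cluster strain to break destructible pieces.
; A radial vector then adds outward linear velocity from the sphere's center, with a culling field confining the push to that radius.
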(event EventBeginPlay
  (bind _fieldsystem (Variables|Default|GetFieldSystem))
  (bind _radialfalloff (Variables|Default|GetRadialFalloff))
  (bind _bombradius (Variables|Default|GetBombRadius))
  (bind _returnvalue (Transformation|GetWorldLocation _bombradius))
  (bind _returnvalue_2 (Components|Sphere|GetScaledSphereRadius _bombradius))
  (bind _returnvalue_3 (Field|SetRadialFalloff _radialfalloff 5e+05 0.0 1.0 0.0 _returnvalue_2 _returnvalue "Field_FallOff_None"))
  (Class|FieldSystemComponent|ApplyPhysicsField _fieldsystem true "Field_ExternalClusterStrain" 0 _returnvalue_3)
  (Class|FieldSystemComponent|ApplyPhysicsField _fieldsystem true "Field_LinearVelocity" 0 (Field|SetCullingField (Variables|Default|GetCullingField) _returnvalue_3 (Field|SetRadialVector (Variables|Default|GetRadialVector) 5e+03 _returnvalue) "Field_Culling_Outside")))

(fn ConstructionScript)