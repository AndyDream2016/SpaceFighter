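; BP_LazerSecondary is a ship component actor that fires a burst of secondary laser shots.
; Fire spawns a BP_LazerProjectile at the actor's transform, passing it the configured look, speed, damage and physics settings plus the parent ship.
; Each shot adds a color-tinted muzzle flash at the Arrow and an optional sound.
; A delayed loop repeats the shot until the rapid-fire round count is reached, then resets the counter.
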(event Custom|Fire
  (bind _lazer_secondary_soundcue (Variables|Default|GetLazer_Secondary_SoundCue))
  (bind _lazer_secondary_color (Variables|Default|GetLazer_Secondary_Color))
  (bind (_r _g _b) (Utilities|Struct|BreakLinearColor _lazer_secondary_color))
  (Game|SpawnActorfromClass "/Game/ScorpionSpaceFighter/Blueprints/ShipComponents/BP_LazerProjectile.BP_LazerProjectile_C" (Math|Transform|MakeTransform (Transformation|GetActorLocation) (Transformation|GetActorRotation) (Math|Conversions|ToVector(Float) (Variables|Default|GetLazer_Secondary_Scale))) "Undefined" 0 (Variables|Default|GetLazer_Secondary_Color) (Variables|Default|GetLazer_Secondary_PhysicsForce) (Variables|Default|GetLazer_Secondary_Explosion%20Scale) (Variables|Default|GetParentShip) (Variables|Default|GetLazer_Secondary_DamageToApply) (Variables|Default|GetLazer_Secondary_PhysicsForce_Multiplier_ForShield) (Variables|Default|GetLazer_Secondary_Speed) (Variables|Default|GetLazer_Secondary_ExplosionBrightness) (Variables|Default|GetLazer_Secondary_PointLightBrightness) (Variables|Default|GetLazer_Secondary_PointLightEnabled) (Variables|Default|GetLazer_Secondary_MaterialGlowIntensity) self :!label _label)
  (bind _returnvalue (Effects|SpawnEmitterAttached "/Game/ScorpionSpaceFighter/Particles/P_ScorpionSpaceFighter_MuzzleFlash.P_ScorpionSpaceFighter_MuzzleFlash" (Variables|Default|GetArrow) "")) ; this is in local space
  (Transformation|SetWorldScale3D _returnvalue (Math|Conversions|ToVector(Float) (Variables|Default|GetMuzzleFlash_Scale)))
  (Effects|Components|ParticleSystem|SetFloatParameter _returnvalue "Color_R" _r)
  (Effects|Components|ParticleSystem|SetFloatParameter _returnvalue "Color_G" _g)
  (Effects|Components|ParticleSystem|SetFloatParameter _returnvalue "Color_B" _b)
  (Variables|Default|SetLazer_Secondary_RapidFire_Count (+ (Variables|Default|GetLazer_Secondary_RapidFire_Count) 1))
  (Utilities|IsValid _lazer_secondary_soundcue
    (:Is%20Valid
      (Audio|PlaySoundatLocation _lazer_secondary_soundcue (Transformation|GetActorLocation)))
    (:Is%20Not%20Valid
      _))
  (Utilities|FlowControl|Delay (Variables|Default|GetLazer_Secondary_RapidFire_Round_Delay))
  (if (>= (Variables|Default|GetLazer_Secondary_RapidFire_Count) (Variables|Default|GetLazer_Secondary_RapidFire_Rounds))
    (Variables|Default|SetLazer_Secondary_RapidFire_Count 0)
    (else
      (goto _label))))

(fn ConstructionScript)