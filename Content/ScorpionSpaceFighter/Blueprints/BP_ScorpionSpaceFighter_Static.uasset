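; Non-drivable, static Scorpion space fighter whose loadout and look are configured through variables applied in the Construction Script.
; Switches on missile and gun settings toggle component visibility, while other options disable collision, pitch the canopy open or remove the tail.
; SetMaterial builds dynamic hull, thruster and cockpit material instances for paint, finish and glow, with thruster settings also driving two spotlights.
; The canopy's inner glass reuses another slot's material to look dark from outside.
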(fn ConstructionScript
  (bind _sm_canopy (Variables|Default|GetSM_Canopy))
  (|ChangeMissiles)
  (|ChangeGuns)
  (Rendering|Material|SetMaterial _sm_canopy 2 (Rendering|Material|GetMaterial _sm_canopy 1)) ; Make inside of Glass Dark (Because it looks better from the outside and we wont be driving this ship)
  (|ToggleCollision)
  (Rendering|Material|SetMaterial)
  (Transformation|SetRelativeRotation (Variables|Default|GetSM_Canopy) (Math|Rotator|MakeRotator 0.0 (Math|Float|Lerp 0.0 9e+01 (Variables|Default|GetGlass_Door_Open?)) 0.0) false false) ; Rotate Canopy Glass
  (if (not (Variables|Default|GetTail))
    (Components|DestroyComponent (Variables|Default|GetSM_Tail))))