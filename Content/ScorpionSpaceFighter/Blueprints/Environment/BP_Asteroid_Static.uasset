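; BP_Asteroid_Static is an environment asteroid actor for the Scorpion space fighter game, with no active event logic.
; Its construction script randomly assigns one of three asteroid meshes and a random world rotation, then stores the mesh's world scale.
; The randomization is unseeded, so the look can change whenever the construction script reruns.
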(event Collision|EventActorBeginOverlap
  (params (OtherActor :type Actor%20Object%20Reference)))

(event EventTick
  (params (DeltaSeconds :type Float%20%28single-precision%29)))

(fn ConstructionScript
  (bind _staticmesh (Variables|Default|GetStaticMesh))
  (bind _output_get (Variables|Default|SetAsteroidType (Math|Random|RandomIntegerinRange 0 2)))
  (switch int _output_get
    (:Default
      (Components|StaticMesh|SetStaticMesh _staticmesh "/Game/ScorpionSpaceFighter/Meshes/Environment/SM_Asteroid_A.SM_Asteroid_A" :!label _label))
    (:0
      (goto _label))
    (:1
      (Components|StaticMesh|SetStaticMesh _staticmesh "/Game/ScorpionSpaceFighter/Meshes/Environment/SM_Asteroid_B.SM_Asteroid_B"))
    (:2
      (Components|StaticMesh|SetStaticMesh _staticmesh "/Game/ScorpionSpaceFighter/Meshes/Environment/SM_Asteroid_E.SM_Asteroid_E")))
  (Transformation|SetWorldRotation (Variables|Default|GetStaticMesh) (Math|Random|RandomRotator true) false false)
  (Variables|Default|SetScale (Transformation|GetWorldScale (Variables|Default|GetStaticMesh))))