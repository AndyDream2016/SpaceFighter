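; Destroyed-asteroid actor that shatters with Chaos physics fields on spawn, then fades out and removes itself.
; The Construction Script keeps one of three asteroid components based on AsteroidType and destroys the others.
; BeginPlay randomly offsets BombRadius in proportion to actor scale, then applies cluster strain and radial velocity fields from that point.
; After Lifetime, a dynamic fadeout material replaces every slot and a timeline drives its opacity before DestroyActor.
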(event EventBeginPlay
  (bind _returnvalue (Transformation|GetActorScale3D))
  (bind _fieldsystem (Variables|Default|GetFieldSystem))
  (bind _bombradius (Variables|Default|GetBombRadius))
  (bind _explosionrandomness (Variables|Default|GetExplosionRandomness))
  (bind _asteroid (Variables|Default|GetAsteroid))
  (bind _returnvalue_2 (Transformation|GetWorldLocation _bombradius))
  (bind _returnvalue_3 (* (.z _returnvalue) _explosionrandomness))
  (bind _returnvalue_4 (* _returnvalue_3 -1.0))
  (bind _returnvalue_5 (Math|Random|RandomFloatinRange _returnvalue_4 _returnvalue_3))
  (Transformation|AddWorldOffset (Variables|Default|GetBombRadius) (Math|Vector|MakeVector _returnvalue_5 _returnvalue_5 _returnvalue_5) false false)
  (Class|FieldSystemComponent|ApplyPhysicsField _fieldsystem true "Field_ExternalClusterStrain" 0 (Field|SetRadialFalloff (Variables|Default|GetRadialFalloff) 5e+05 0.0 1.0 0.0 (Components|Sphere|GetScaledSphereRadius _bombradius) _returnvalue_2 "Field_FallOff_None"))
  (Class|FieldSystemComponent|ApplyPhysicsField _fieldsystem true "Field_LinearVelocity" 0 (Field|SetRadialVector (Variables|Default|GetRadialVector) 5e+02 _returnvalue_2))
  (Utilities|FlowControl|Delay (Variables|Default|GetLifetime))
  (bind _returnvalue_6 (Rendering|Material|CreateDynamicMaterialInstance "/Game/ScorpionSpaceFighter/Materials/Environment/M_Asteroid_Fadeout.M_Asteroid_Fadeout" "None" "None" :!class /Script/Engine.KismetMaterialLibrary))
  (Variables|Default|SetFadeout_Mat _returnvalue_6)
  (for _index (range 0 (Rendering|Material|GetNumMaterials _asteroid))
    (Rendering|Material|SetMaterial _asteroid _index (Variables|Default|GetFadeout_Mat)))
  (bind _opacity (Timeline|Timeline_0 PlayFromStart)
    (:Update
      (Rendering|Material|SetScalarParameterValue (Variables|Default|GetFadeout_Mat) "Opacity" _opacity :!class /Script/Engine.MaterialInstanceDynamic))
    (:Finished
      (Actor|DestroyActor))))

(fn ConstructionScript
  (bind _asteroid_e (Variables|Default|GetAsteroid_E))
  (switch int (Variables|Default|GetAsteroidType)
    (:0
      (Components|DestroyComponent _asteroid_e)
      (Variables|Default|SetAsteroid (Variables|Default|GetAsteroid_A)))
    (:1
      (Components|DestroyComponent _asteroid_e)
      (Variables|Default|SetAsteroid (Variables|Default|GetAsteroid_B)))
    (:2
      (Components|DestroyComponent (Variables|Default|GetAsteroid_B))
      (Variables|Default|SetAsteroid (Variables|Default|GetAsteroid_E)))))