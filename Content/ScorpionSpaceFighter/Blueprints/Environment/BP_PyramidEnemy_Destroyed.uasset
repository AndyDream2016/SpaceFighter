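; BP_PyramidEnemy_Destroyed is the shattering wreck of a pyramid enemy that fades away after breaking apart.
; On BeginPlay it randomly offsets a bomb radius scaled by actor size, then applies Chaos field strain and radial velocity from it to fracture and scatter the pieces.
; After a lifetime delay it swaps in dynamic fadeout materials for both slots, animates their opacity on a timeline, then destroys itself.
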(event EventBeginPlay
  (bind _returnvalue (Transformation|GetActorScale3D))
  (bind _fieldsystem (Variables|Default|GetFieldSystem))
  (bind _bombradius (Variables|Default|GetBombRadius))
  (bind _dsm_pyramidenemy (Variables|Default|GetDSM_PyramidEnemy))
  (bind _explosionrandomness (Variables|Default|GetExplosionRandomness))
  (bind _returnvalue_2 (Transformation|GetWorldLocation _bombradius))
  (bind _returnvalue_3 (* (.z _returnvalue) _explosionrandomness))
  (bind _returnvalue_4 (* _returnvalue_3 -1.0))
  (bind _returnvalue_5 (Math|Random|RandomFloatinRange _returnvalue_4 _returnvalue_3))
  (Transformation|AddWorldOffset (Variables|Default|GetBombRadius) (Math|Vector|MakeVector _returnvalue_5 _returnvalue_5 _returnvalue_5) false false)
  (Class|FieldSystemComponent|ApplyPhysicsField _fieldsystem true "Field_ExternalClusterStrain" 0 (Field|SetRadialFalloff (Variables|Default|GetRadialFalloff) 5e+05 0.0 1.0 0.0 (Components|Sphere|GetScaledSphereRadius _bombradius) _returnvalue_2 "Field_FallOff_None"))
  (Class|FieldSystemComponent|ApplyPhysicsField _fieldsystem true "Field_LinearVelocity" 0 (Field|SetRadialVector (Variables|Default|GetRadialVector) 5e+02 _returnvalue_2))
  (Utilities|FlowControl|Delay (Variables|Default|GetLifetime))
  (bind _returnvalue_6 (Rendering|Material|CreateDynamicMaterialInstance "/Game/ScorpionSpaceFighter/Materials/Environment/M_PyramidEnemy_Fadeout.M_PyramidEnemy_Fadeout" "None" "None" :!class /Script/Engine.KismetMaterialLibrary))
  (bind _output_get (Variables|Default|SetFadeout_Mat _returnvalue_6))
  (Rendering|Material|SetMaterial _dsm_pyramidenemy 0 _output_get)
  (bind _returnvalue_7 (Rendering|Material|CreateDynamicMaterialInstance "/Game/ScorpionSpaceFighter/Materials/Environment/MI_PyramidEnemy_Fadeout_B.MI_PyramidEnemy_Fadeout_B" "None" "None" :!class /Script/Engine.KismetMaterialLibrary))
  (bind _output_get_2 (Variables|Default|SetFadeout_Mat_Inner _returnvalue_7))
  (Rendering|Material|SetMaterial _dsm_pyramidenemy 1 _output_get_2)
  (bind _opacity (Timeline|FadeOut PlayFromStart)
    (:Update
      (Rendering|Material|SetScalarParameterValue (Variables|Default|GetFadeout_Mat) "Opacity" _opacity :!class /Script/Engine.MaterialInstanceDynamic))
    (:Finished
      (Actor|DestroyActor))))

(fn ConstructionScript)